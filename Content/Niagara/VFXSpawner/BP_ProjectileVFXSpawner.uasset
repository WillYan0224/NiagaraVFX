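; BP_ProjectileVFXSpawner is a spawner actor that repeatedly fires projectiles carrying configurable Niagara effects.
; On BeginPlay it spawns one immediately, then a looping timer spawns a BP_Projectile_Master at its location every ProjectileSpawnGap.
; Each projectile receives the spawner's muzzle, main and hit impact VFX, an X-axis velocity from ProjectileSpeed, an effect offset and a destroy delay.
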(event `self.ReceiveBeginPlay`
  (`self.SpawnProjectileVFX`)
  (`KismetSystemLibrary.K2_SetTimerDelegate` (delegate `SpawnProjectileVFX`) (`self.ProjectileSpawnGap`) true))

(event `SpawnProjectileVFX`
  (bind _returnvalue (`|SpawnActorFromClass` "/Game/Niagara/VFXSpawner/BP_Projectile_Master.BP_Projectile_Master_C" (`KismetMathLibrary.MakeTransform` (`self.K2_GetActorLocation`)) "Undefined" "MultiplyWithRoot" null null))
  (bind _output_get (set `self.SpawnProjectile` _returnvalue))
  (`/Engine/EditorBlueprintResources/StandardMacros.IsValid` _output_get
    (:`Is Valid`
      (`|ExecutionSequence`
        (:`then_0`
          ;[1 1 1] Setting VFX Niagara Variables
          (set `/Game/Niagara/VFXSpawner/BP_Projectile_Master.MuzzleVFX` (`self.Muzzle VFX`) (`self.SpawnProjectile`))
          (`NiagaraComponent.SetAsset` (`/Game/Niagara/VFXSpawner/BP_Projectile_Master.ProjectileVFXComponent` (`self.SpawnProjectile`)) (`self.MainProjectileVFX`) true)
          (set `/Game/Niagara/VFXSpawner/BP_Projectile_Master.HitImpactVFX` (`self.Hit Impact VFX`) (`self.SpawnProjectile`)))
        (:`then_1`
          ;[1 1 1] Setting Projectile Speed
          (set `MovementComponent.Velocity` (* (`self.ProjectileSpeed`) (1.0 0.0 0.0)) (`/Game/Niagara/VFXSpawner/BP_Projectile_Master.ProjectileMovementComponent` (`self.SpawnProjectile`))))
        (:`then_2`
          ;[1 1 1] Setting Offset Of Muzzle and Hit Impact
          (set `/Game/Niagara/VFXSpawner/BP_Projectile_Master.MuzzleHitImpactOffset` (`self.Muzzle Hit Impact Offset`) (`self.SpawnProjectile`))
          ;[1 1 1] Setting Destory Delay Of Projectile Actor
          (set `/Game/Niagara/VFXSpawner/BP_Projectile_Master.ProjectileDestoryDelay` (`self.Projectile Destory Delay`) (`self.SpawnProjectile`)))))))

(fn `UserConstructionScript`)