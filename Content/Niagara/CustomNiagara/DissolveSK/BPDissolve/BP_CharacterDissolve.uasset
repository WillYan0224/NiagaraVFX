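; Character dissolve actor that plays a material and Niagara dissolve effect on its skeletal mesh when a BP_Spawn actor enters its box trigger.
; On overlap, it creates dynamic instances of the two Manny dissolve materials and assigns them to the mesh.
; A timeline drives their dissolve scalar while NS_BPDissolve spawns attached to the mesh.
; Leaving the box reverses the timeline.
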(event `self.Box.OnComponentBeginOverlap`
  (params (OverlappedComponent :type "PrimitiveComponent Object Reference") (OtherActor :type "Actor Object Reference") (OtherComp :type "PrimitiveComponent Object Reference") (OtherBodyIndex :type Integer) (bFromSweep :type Boolean) (SweepResult :type "HitResult Structure (by ref)"))
  (cast `/Game/Blueprints/BP_Spawn` OtherActor)
  (`|ExecutionSequence`
    (:`then_0`
      ;[1 1 1] Creating Dynaminc instances
      (bind _returnvalue (`KismetMaterialLibrary.CreateDynamicMaterialInstance` "/Game/Niagara/CustomNiagara/DissolveSK/BPDissolve/MI_Manny_01_BPDissolve.MI_Manny_01_BPDissolve"))
      (set `self.Created_Dy_MI_Manny01` _returnvalue)
      (bind _returnvalue_2 (`KismetMaterialLibrary.CreateDynamicMaterialInstance` "/Game/Niagara/CustomNiagara/DissolveSK/BPDissolve/MI_Manny_02_BPDissolve.MI_Manny_02_BPDissolve"))
      (set `self.Created_Dy_MI_Manny02` _returnvalue_2))
    (:`then_1`
      ;[1 1 1] Setting new material for character
      (`PrimitiveComponent.SetMaterial` (`self.SkeletalMesh`) 0 (`self.Created_Dy_MI_Manny01`))
      (`PrimitiveComponent.SetMaterial` (`self.SkeletalMesh`) 1 (`self.Created_Dy_MI_Manny02`)))
    (:`then_2`
      ;[1 1 1] Timeline Control dissolve amount
      (bind (_direction _dissolvetrack) (`Timeline|DissolveTimeline` :!via `PlayFromStart` :!label _label)
        (:`Update`
          (`MaterialInstanceDynamic.SetScalarParameterValue` (`self.Created_Dy_MI_Manny01`) "DissolveAmout" _dissolvetrack)
          (`MaterialInstanceDynamic.SetScalarParameterValue` (`self.Created_Dy_MI_Manny02`) "DissolveAmout" _dissolvetrack))))
    (:`then_3`
      (`NiagaraFunctionLibrary.SpawnSystemAttached` "/Game/Niagara/CustomNiagara/DissolveSK/NS_BPDissolve.NS_BPDissolve" (`self.SkeletalMesh`) "None" (0.0 0.0 0.0) (struct) "SnapToTarget"))))

(event `self.Box.OnComponentEndOverlap`
  (params (OverlappedComponent :type "PrimitiveComponent Object Reference") (OtherActor :type "Actor Object Reference") (OtherComp :type "PrimitiveComponent Object Reference") (OtherBodyIndex :type Integer))
  (cast `/Game/Blueprints/BP_Spawn` OtherActor)
  (goto _label :!via `Reverse`))

(fn `UserConstructionScript`)